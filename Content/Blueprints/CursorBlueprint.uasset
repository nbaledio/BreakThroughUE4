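; Cursor actor, apparently for a two-player character select, that records the hovered character's name on overlap and animates a linked render sprite.
; Overlap plays the P1 or P2 slide timeline based on Side, and ending overlap clears the name.
; Slide timelines move the render with a masked material, while a separately triggered fade timeline drives sprite color with a translucent one.
; Helper functions assign the render, replay animations and reset color.
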(event `self.ReceiveActorBeginOverlap`
  (params (OtherActor :type "Actor Object Reference"))
  ;[1 1 1] Collision Detection
  (set `self.HoveredCharacter` (`KismetSystemLibrary.GetDisplayName` OtherActor))
  (if (`KismetStringLibrary.EqualEqual_StrStr` (`self.Side`) "Left")
    (`self.PlayP1RenderSlide`)
    (else
      (`self.PlayP2RenderSlide`))))

(event `self.ReceiveActorEndOverlap`
  (params (OtherActor :type "Actor Object Reference"))
  ;[1 1 1] Collision Detection
  (set `self.HoveredCharacter` ""))

(fn `PlayP1RenderSlide`
  (`TimelineComponent.PlayFromStart` (`self.P1RenderSlide`)))

(fn `PlayP2RenderSlide`
  (`TimelineComponent.PlayFromStart` (`self.P2RenderSlide`)))

(fn `PlayRenderFadeAway`
  (`TimelineComponent.PlayFromStart` (`self.RenderFadeAway`)))

(fn `PlayRenderSlide`
  (if (`KismetStringLibrary.EqualEqual_StrStr` (`self.Side`) "Left")
    (`self.PlayP1RenderSlide`)
    (else
      (`self.PlayP2RenderSlide`))))

(fn `ResetSpriteColor`
  (`PaperSpriteComponent.SetSpriteColor` (`PaperSpriteActor.RenderComponent` (`self.Render`)) (struct :`R` 1.0 :`G` 1.0 :`B` 1.0 :`A` 1.0)))

(fn `SetRender`
  (params (Render :type "PaperSpriteActor Object Reference"))
  (set `self.Render` Render))

(fn `UserConstructionScript`)